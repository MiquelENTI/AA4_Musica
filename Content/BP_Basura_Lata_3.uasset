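; BP_Basura_Lata_3 is a trash can prop that marks itself when it is the first-person player's focused actor.
; Each Tick it casts the player character to BP_FirstPersonCharacter and compares FocusedActorName against its own hardcoded name string.
; It sets the StaticMesh custom depth stencil to 1 on a match and 0 otherwise, which suggests a post-process highlight.
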(event EventBeginPlay)

(event Collision|EventActorBeginOverlap
  (params (OtherActor :type Actor%20Object%20Reference)))

(event EventTick
  (params (DeltaSeconds :type Float%20%28single-precision%29))
  (bind _asbp_first_person_character (Utilities|Casting|CastToBP_FirstPersonCharacter (Game|GetPlayerCharacter 0)))
  (Utilities|FlowControl|Sequence
    (:then_0
      (if (Utilities|Enum|Equal(Enum) "Basura_Lata_3" (Variables|/Game/FirstPerson/Blueprints/BP_FirstPersonCharacter.BP_FirstPersonCharacter_C|GetFocused%20Actor%20Name _asbp_first_person_character))
        (Rendering|SetCustomDepthStencilValue (Variables|Default|GetStaticMesh) 1)
        (else
          (Rendering|SetCustomDepthStencilValue (Variables|Default|GetStaticMesh) 0))))))

(fn ConstructionScript)